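; BP_HeadTarget is a head target actor that travels along the spline track of the level's BP_ShootingBooth.
; On BeginPlay it finds the booth and caches its spline.
; MoveObject plays a timeline from TrackPosition at a rate set by TimeToComplete, mapping its alpha to spline distance to set location and rotation.
; Setters expose start position and duration; location is read in world space, rotation in local space.
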(event `self.ReceiveBeginPlay`
  (bind _returnvalue (`GameplayStatics.GetActorOfClass` "/Game/GameBooths/ShootingBooth/BP_ShootingBooth.BP_ShootingBooth_C"))
  (`/Engine/EditorBlueprintResources/StandardMacros.IsValid` _returnvalue
    (:`Is Valid`
      (bind _splineoutput (`/Game/GameBooths/ShootingBooth/BP_ShootingBooth.GetSplineComponent` _returnvalue))
      (set `self.SplineRef` _splineoutput))))

(event `Move Object`
  (bind _splineref (`self.SplineRef`))
  (bind _movementtimeline (`self.MovementTimeline`))
  (`TimelineComponent.SetPlayRate` _movementtimeline (/ 1.0 (`self.TimeToComplete`)))
  (`TimelineComponent.SetNewTime` _movementtimeline (`self.TrackPosition`))
  (bind (_direction _move_track) (`Timeline|MovementTimeline`)
    (:`Update`
      (bind _returnvalue (`KismetMathLibrary.Lerp` 0.0 (`SplineComponent.GetSplineLength` (`self.SplineRef`)) _move_track))
      (`self.K2_SetActorTransform` (`KismetMathLibrary.MakeTransform` (`SplineComponent.GetLocationAtDistanceAlongSpline` _splineref _returnvalue "World") (`SplineComponent.GetRotationAtDistanceAlongSpline` _splineref _returnvalue "Local"))))))

(fn `SetTimeToComplete`
  (params (Time :type "Float (double-precision)"))
  (set `self.TimeToComplete` Time))

(fn `SetTrackPosition`
  (params (NewTrackPosition :type "Float (double-precision)"))
  (set `self.TrackPosition` NewTrackPosition))

(fn `UserConstructionScript`)