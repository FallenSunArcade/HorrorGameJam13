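; Monster duck enemy that transforms when the player first enters its detection sphere, then chases and attacks.
; Chained timelines grow legs, neck, beak, teeth and eyes through morph targets, alongside a MonsterValue material parameter.
; A looping timer then re-issues AI moves and sets Attacking from proximity; HitEnemy damages a player inside the attack collision.
; At zero health it stops moving and, after a delay, one timeline animates all morphs.
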(event `self.ReceiveBeginPlay`
  (bind _returnvalue (`PrimitiveComponent.CreateDynamicMaterialInstance` (`self.Mesh`) 0 null "None"))
  (bind _asbp_player (cast `/Game/BP_Player` (`GameplayStatics.GetPlayerCharacter` 0)))
  (set `self.Player` _asbp_player))

(event `Spawn`
  (bind _mesh (`self.Mesh`))
  (bind (_direction _newtrack_0) (`Timeline|Timeline`)
    (:`Update`
      (`SkeletalMeshComponent.SetMorphTarget` (`self.Mesh`) "leg-f1" _newtrack_0 true))
    (:`Finished`
      (`KismetSystemLibrary.Delay` 0.5)
      (bind (_direction_2 _newtrack_0_2) (`Timeline|Timeline_0`)
        (:`Update`
          (`SkeletalMeshComponent.SetMorphTarget` (`self.Mesh`) "leg-b1" _newtrack_0_2 true))
        (:`Finished`
          (`KismetSystemLibrary.Delay` 0.5)
          (bind (_direction_3 _newtrack_0_3) (`Timeline|Timeline_1`)
            (:`Update`
              (`SkeletalMeshComponent.SetMorphTarget` (`self.Mesh`) "leg-f2" _newtrack_0_3 true)
              (bind (_direction_4 _newtrack_0_4) (`Timeline|Timeline_2`)
                (:`Update`
                  (`SkeletalMeshComponent.SetMorphTarget` (`self.Mesh`) "leg-b2" _newtrack_0_4 true)
                  (bind (_direction_5 _newtrack_0_5) (`Timeline|Timeline_3`)
                    (:`Update`
                      (`SkeletalMeshComponent.SetMorphTarget` (`self.Mesh`) "leg-m1" _newtrack_0_5 true))
                    (:`Finished`
                      (bind (_direction_6 _newtrack_0_6) (`Timeline|Timeline_4`)
                        (:`Update`
                          (`SkeletalMeshComponent.SetMorphTarget` (`self.Mesh`) "leg-m2" _newtrack_0_6 true)
                          (`MaterialInstanceDynamic.SetScalarParameterValue` (stale `self.ReceiveBeginPlay` _returnvalue) "MonsterValue" _newtrack_0_6)
                          (`SkeletalMeshComponent.SetMorphTarget` _mesh "longneck" _newtrack_0_6 true)
                          (`SkeletalMeshComponent.SetMorphTarget` _mesh "beak" _newtrack_0_6 true)
                          (`SkeletalMeshComponent.SetMorphTarget` _mesh "teeth" _newtrack_0_6 true)
                          (`SkeletalMeshComponent.SetMorphTarget` _mesh "eyes" _newtrack_0_6 true))
                        (:`Finished`
                          (`Timeline|Timeline_5`
                            (:`Finished`
                              (`KismetSystemLibrary.Delay` 1.0)
                              (set `self.FullySpawned` true)
                              (`KismetSystemLibrary.K2_SetTimer` null "FollowPlayer" 0.2 true))))))))))))))))

(event `self.PlayerDetectionSphere.OnComponentBeginOverlap`
  (params (OverlappedComponent :type "PrimitiveComponent Object Reference") (OtherActor :type "Actor Object Reference") (OtherComp :type "PrimitiveComponent Object Reference") (OtherBodyIndex :type Integer) (bFromSweep :type Boolean) (SweepResult :type "HitResult Structure (by ref)"))
  ;[1 1 1] PlayerNearby
  (if (== (`|GetArrayItem` (`Actor.Tags` OtherActor)) "Player")
    (set `self.PlayerNearby` true)
    (if (not (`self.Spawning`))
      (`/Engine/EditorBlueprintResources/StandardMacros.DoOnce` false
        (:`Completed`
          (`self.Spawn`)
          (set `self.Spawning` true))))))

(event `FollowPlayer`
  ;[1 1 1] Follow Player
  (if (`self.PlayerNearby`)
    (set `self.Attacking` true)
    (else
      (set `self.Attacking` false)))
  (`|AIMoveTo` self (`self.K2_GetActorLocation` (`self.Player`)) null 150.0))

(event `self.PlayerDetectionSphere.OnComponentEndOverlap`
  (params (OverlappedComponent :type "PrimitiveComponent Object Reference") (OtherActor :type "Actor Object Reference") (OtherComp :type "PrimitiveComponent Object Reference") (OtherBodyIndex :type Integer))
  (if (== (`|GetArrayItem` (`Actor.Tags` OtherActor)) "Player")
    (set `self.PlayerNearby` false)))

(event `HitEnemy`
  (if (`self.PlayerInAttackCollision`)
    (`GameplayStatics.ApplyDamage` (`self.Player`) 5.0)))

(event `self.AttackHitCollision.OnComponentBeginOverlap`
  (params (OverlappedComponent :type "PrimitiveComponent Object Reference") (OtherActor :type "Actor Object Reference") (OtherComp :type "PrimitiveComponent Object Reference") (OtherBodyIndex :type Integer) (bFromSweep :type Boolean) (SweepResult :type "HitResult Structure (by ref)"))
  (if (== (`|GetArrayItem` (`Actor.Tags` OtherActor)) "Player")
    (set `self.PlayerInAttackCollision` true)))

(event `self.AttackHitCollision.OnComponentEndOverlap`
  (params (OverlappedComponent :type "PrimitiveComponent Object Reference") (OtherActor :type "Actor Object Reference") (OtherComp :type "PrimitiveComponent Object Reference") (OtherBodyIndex :type Integer))
  (if (== (`|GetArrayItem` (`Actor.Tags` OtherActor)) "Player")
    (set `self.PlayerInAttackCollision` false)))

(event `self.ReceiveAnyDamage`
  (params (Damage :type "Float (single-precision)") (DamageType :type "DamageType Object Reference") (InstigatedBy :type "Controller Object Reference") (DamageCauser :type "Actor Object Reference"))
  (bind _mesh (`self.Mesh`))
  (bind _mesh_2 (`self.Mesh`))
  (bind _mesh_3 (`self.Mesh`))
  (bind _output_get (set `self.MonsterHealth` (- (`self.MonsterHealth`) Damage)))
  (if (<= _output_get 0.0)
    (set `self.MonsterDead` true)
    (`CharacterMovementComponent.SetMovementMode` (`self.CharacterMovement`) "MOVE_None" 0)
    (`KismetSystemLibrary.Delay` 2.0)
    (bind (_direction _newtrack_0) (`Timeline|Timeline_6`)
      (:`Update`
        (`SkeletalMeshComponent.SetMorphTarget` (`self.Mesh`) "leg-f1" _newtrack_0 true)
        (`SkeletalMeshComponent.SetMorphTarget` (`self.Mesh`) "leg-b1" _newtrack_0 true)
        (`SkeletalMeshComponent.SetMorphTarget` (`self.Mesh`) "leg-f2" _newtrack_0 true)
        (`SkeletalMeshComponent.SetMorphTarget` _mesh_2 "leg-b2" _newtrack_0 true)
        (`SkeletalMeshComponent.SetMorphTarget` _mesh_2 "leg-m1" _newtrack_0 true)
        (`SkeletalMeshComponent.SetMorphTarget` _mesh_3 "leg-m2" _newtrack_0 true)
        (`SkeletalMeshComponent.SetMorphTarget` _mesh_3 "longneck" _newtrack_0 true)
        (`SkeletalMeshComponent.SetMorphTarget` _mesh "beak" _newtrack_0 true)
        (`SkeletalMeshComponent.SetMorphTarget` _mesh "teeth" _newtrack_0 true)
        (`SkeletalMeshComponent.SetMorphTarget` _mesh "eyes" _newtrack_0 true)))))

(fn `UserConstructionScript`)