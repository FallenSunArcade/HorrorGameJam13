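; Monster duck actor that transforms through morph targets when an actor tagged "Player" overlaps its R component.
; The overlap calls Spawn and sets a Spawned flag, which nothing here reads.
; Spawn drives chained timelines that morph six legs, then the neck, beak, teeth and eyes along with the last leg.
; Early stages are separated by delays, while some later timelines start from the previous one's Update, so they overlap.
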(event `Spawn`
  (bind _mesh (`self.Mesh`))
  (bind (_direction _newtrack_0) (`Timeline|Timeline`)
    (:`Update`
      (`SkeletalMeshComponent.SetMorphTarget` (`self.Mesh`) "leg-f1" _newtrack_0 true))
    (:`Finished`
      (`KismetSystemLibrary.Delay` 0.5)
      (bind (_direction_2 _newtrack_0_2) (`Timeline|Timeline_0`)
        (:`Update`
          (`SkeletalMeshComponent.SetMorphTarget` (`self.Mesh`) "leg-b1" _newtrack_0_2 true))
        (:`Finished`
          (`KismetSystemLibrary.Delay` 0.5)
          (bind (_direction_3 _newtrack_0_3) (`Timeline|Timeline_1`)
            (:`Update`
              (`SkeletalMeshComponent.SetMorphTarget` (`self.Mesh`) "leg-f2" _newtrack_0_3 true)
              (bind (_direction_4 _newtrack_0_4) (`Timeline|Timeline_2`)
                (:`Update`
                  (`SkeletalMeshComponent.SetMorphTarget` (`self.Mesh`) "leg-b2" _newtrack_0_4 true)
                  (bind (_direction_5 _newtrack_0_5) (`Timeline|Timeline_3`)
                    (:`Update`
                      (`SkeletalMeshComponent.SetMorphTarget` (`self.Mesh`) "leg-m1" _newtrack_0_5 true))
                    (:`Finished`
                      (bind (_direction_6 _newtrack_0_6) (`Timeline|Timeline_4`)
                        (:`Update`
                          (`SkeletalMeshComponent.SetMorphTarget` (`self.Mesh`) "leg-m2" _newtrack_0_6 true)
                          (`SkeletalMeshComponent.SetMorphTarget` _mesh "longneck" _newtrack_0_6 true)
                          (`SkeletalMeshComponent.SetMorphTarget` _mesh "beak" _newtrack_0_6 true)
                          (`SkeletalMeshComponent.SetMorphTarget` _mesh "teeth" _newtrack_0_6 true)
                          (`SkeletalMeshComponent.SetMorphTarget` _mesh "eyes" _newtrack_0_6 true))
                        (:`Finished`
                          (`Timeline|Timeline_5`))))))))))))))

(event `self.ReceiveBeginPlay`)

(event `self.r.OnComponentBeginOverlap`
  (params (OverlappedComponent :type "PrimitiveComponent Object Reference") (OtherActor :type "Actor Object Reference") (OtherComp :type "PrimitiveComponent Object Reference") (OtherBodyIndex :type Integer) (bFromSweep :type Boolean) (SweepResult :type "HitResult Structure (by ref)"))
  (if (== (`|GetArrayItem` (`Actor.Tags` OtherActor)) "Player")
    (`self.Spawn`)
    (set `self.Spawned` true)))

(fn `UserConstructionScript`)