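; Mole enemy that spawns when the player enters its range sphere, then chases and attacks them, turning to face them every tick.
; The first overlap raises a Spawn flag, waits out a delay, then starts a looping timer that calls AIMoveTo toward the player.
; Reaching the player holds an Attacking flag briefly, pausing new move requests.
; Both hand colliders apply damage only while DamageState is set, which happens outside this graph.
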(event `self.ReceiveBeginPlay`
  (bind _asbp_player (cast `/Game/BP_Player` (`GameplayStatics.GetPlayerCharacter` 0)))
  (set `self.Player` _asbp_player))

(event `self.ReceiveTick`
  (params (DeltaSeconds :type "Float (single-precision)"))
  (`self.K2_SetActorRotation` (`KismetMathLibrary.FindLookAtRotation` (`self.K2_GetActorLocation`) (`self.K2_GetActorLocation` (`self.Player`)))))

(event `self.RangeDetectionSphere.OnComponentBeginOverlap`
  (params (OverlappedComponent :type "PrimitiveComponent Object Reference") (OtherActor :type "Actor Object Reference") (OtherComp :type "PrimitiveComponent Object Reference") (OtherBodyIndex :type Integer) (bFromSweep :type Boolean) (SweepResult :type "HitResult Structure (by ref)"))
  (if (== (`|GetArrayItem` (`Actor.Tags` OtherActor)) "Player")
    (`/Engine/EditorBlueprintResources/StandardMacros.DoOnce` false
      (:`Completed`
        (set `self.Spawn` true)
        (`KismetSystemLibrary.PrintString` "SPAWN")
        (`KismetSystemLibrary.Delay` 4.0)
        (`KismetSystemLibrary.K2_SetTimer` null "FollowPlayer" 0.1 true)
        (set `self.Spawn` false)))))

(event `FollowPlayer`
  (if (not (`self.Attacking`))
    (`|AIMoveTo` self (`SceneComponent.K2_GetComponentLocation` (`Actor.RootComponent` (`self.Player`))) null 150.0
      (:`OnSuccess`
        (set `self.Attacking` true)
        (`KismetSystemLibrary.Delay` 2.5)
        (set `self.Attacking` false)))))

(event `self.LefttHand_collider.OnComponentBeginOverlap`
  (params (OverlappedComponent :type "PrimitiveComponent Object Reference") (OtherActor :type "Actor Object Reference") (OtherComp :type "PrimitiveComponent Object Reference") (OtherBodyIndex :type Integer) (bFromSweep :type Boolean) (SweepResult :type "HitResult Structure (by ref)"))
  (if (== (`|GetArrayItem` (`Actor.Tags` OtherActor)) "Player")
    (if (`self.DamageState`)
      (`GameplayStatics.ApplyDamage` OtherActor 10.0))))

(event `self.RightHand_collider.OnComponentBeginOverlap`
  (params (OverlappedComponent :type "PrimitiveComponent Object Reference") (OtherActor :type "Actor Object Reference") (OtherComp :type "PrimitiveComponent Object Reference") (OtherBodyIndex :type Integer) (bFromSweep :type Boolean) (SweepResult :type "HitResult Structure (by ref)"))
  (if (== (`|GetArrayItem` (`Actor.Tags` OtherActor)) "Player")
    (if (`self.DamageState`)
      (`GameplayStatics.ApplyDamage` OtherActor 10.0))))

(fn `UserConstructionScript`)