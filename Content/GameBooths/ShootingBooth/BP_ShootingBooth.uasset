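; BP_ShootingBooth is a shooting gallery booth that populates a spline track with moving targets.
; On BeginPlay it spawns a BP_ShootingTarget at each StartingPoints time along the spline.
; Each target receives its track position and a shared fixed completion time, then starts moving.
; Getters expose the spline, shooting position and dialog component to other objects.
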(event `self.ReceiveBeginPlay`
  (for _array_element (`self.StartingPoints`)
    (bind _output_get (set `self.CurrentPoint` _array_element))
    (bind _returnvalue (`|SpawnActorFromClass` "/Game/Assets/NormalDuck/BP_ShootingTarget.BP_ShootingTarget_C" (`SplineComponent.GetTransformAtTime` (`self.Spline`) _output_get "World" false false) "Undefined" "OverrideRootScale" null null))
    (`/Game/Assets/NormalDuck/BP_ShootingTarget.SetTrackPosition` _returnvalue (`self.CurrentPoint`))
    (`/Game/Assets/NormalDuck/BP_ShootingTarget.SetTimeToComplete` _returnvalue 10.0)
    (`/Game/Assets/NormalDuck/BP_ShootingTarget.Move Object` _returnvalue)))

(fn `GetDialogComponent`
  (returns (DialogComponent :type "/Game/Core/DialogSystem/BP_DialogComponent Object Reference"))
  (return (`self.BP_DialogComponent`)))

(fn `GetShootingPosition`
  (returns (ShootingPosition :type "SceneComponent Object Reference"))
  (return (`self.ShootingPosition`)))

(fn `GetSplineComponent`
  (returns (SplineOutput :type "SplineComponent Object Reference"))
  (return (`self.Spline`)))

(fn `UserConstructionScript`)