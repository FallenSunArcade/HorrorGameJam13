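; Woman character Blueprint that gives its Mother3 mesh a randomized body, face, hair and outfit, with animated facial expressions.
; BeginPlay randomizes scale and many morph target weights, then creates a dynamic Woman_Mat instance with a random pants toggle and two random colors.
; The NewShape event jumps back into that same chain to re-roll the look.
; Tick keeps three nested timelines playing, driving the eyesclosed, eyessmall and happy morphs.
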(event `self.ReceiveTick`
  (params (DeltaSeconds :type "Float (single-precision)"))
  (bind (_direction _newtrack_0) (`Timeline|Timeline`)
    (:`Update`
      (`SkeletalMeshComponent.SetMorphTarget` (`self.mother3`) "eyesclosed" _newtrack_0 true)
      (bind (_direction_2 _newtrack_0_2) (`Timeline|Timeline_0`)
        (:`Update`
          (`SkeletalMeshComponent.SetMorphTarget` (`self.mother3`) "eyessmall" _newtrack_0_2 true)
          (bind (_direction_3 _newtrack_0_3) (`Timeline|Timeline_1`)
            (:`Update`
              (`SkeletalMeshComponent.SetMorphTarget` (`self.mother3`) "happy" _newtrack_0_3 true))))))))

(event `self.ReceiveBeginPlay`
  (`SceneComponent.SetWorldScale3D` (`self.mother3`) (`KismetMathLibrary.MakeVector` (`KismetMathLibrary.RandomFloatInRange` 0.65 0.7) (`KismetMathLibrary.RandomFloatInRange` 0.65 0.7) (`KismetMathLibrary.RandomFloatInRange` 0.65 0.7)) :!label _label)
  (`SkeletalMeshComponent.SetMorphTarget` (`self.mother3`) "size" (`KismetMathLibrary.RandomFloatInRange` 0.0 1.0) true)
  (`SkeletalMeshComponent.SetMorphTarget` (`self.mother3`) "breasts" (`KismetMathLibrary.RandomFloatInRange` 0.0 1.0) true)
  (`SkeletalMeshComponent.SetMorphTarget` (`self.mother3`) "shirt" (`KismetMathLibrary.RandomFloatInRange` 0.0 1.0) true)
  (`SkeletalMeshComponent.SetMorphTarget` (`self.mother3`) "feet" (`KismetMathLibrary.RandomFloatInRange` 0.0 1.0) true)
  (`SkeletalMeshComponent.SetMorphTarget` (`self.mother3`) "neck" (`KismetMathLibrary.RandomFloatInRange` 0.0 1.0) true)
  (`SkeletalMeshComponent.SetMorphTarget` (`self.mother3`) "pointyshoe" (`KismetMathLibrary.RandomFloatInRange` 0.0 1.0) true)
  (`SkeletalMeshComponent.SetMorphTarget` (`self.mother3`) "Happy" (`KismetMathLibrary.RandomFloatInRange` 0.0 1.0) true)
  (`SkeletalMeshComponent.SetMorphTarget` (`self.mother3`) "Sad" (`KismetMathLibrary.RandomFloatInRange` 0.0 0.5) true)
  (`SkeletalMeshComponent.SetMorphTarget` (`self.mother3`) "angry" (`KismetMathLibrary.RandomFloatInRange` 0.0 1.0) true)
  (`SkeletalMeshComponent.SetMorphTarget` (`self.mother3`) "FaceShape" (`KismetMathLibrary.RandomFloatInRange` 0.0 0.3) true)
  (`SkeletalMeshComponent.SetMorphTarget` (`self.mother3`) "Key 19" (`KismetMathLibrary.RandomFloatInRange` 0.0 0.3) true)
  (`SkeletalMeshComponent.SetMorphTarget` (`self.mother3`) "Key 20" (`KismetMathLibrary.RandomFloatInRange` 0.0 0.3) true)
  (`SkeletalMeshComponent.SetMorphTarget` (`self.mother3`) "Key 21" (`KismetMathLibrary.RandomFloatInRange` 0.0 0.3) true)
  (`SkeletalMeshComponent.SetMorphTarget` (`self.mother3`) "Key 22" (`KismetMathLibrary.RandomFloatInRange` 0.0 0.3) true)
  (`SkeletalMeshComponent.SetMorphTarget` (`self.mother3`) "Key 23" (`KismetMathLibrary.RandomFloatInRange` 0.0 0.3) true)
  (`SkeletalMeshComponent.SetMorphTarget` (`self.mother3`) "Key 24" (`KismetMathLibrary.RandomFloatInRange` 0.0 0.3) true)
  (`SkeletalMeshComponent.SetMorphTarget` (`self.mother3`) "Key 25" (`KismetMathLibrary.RandomFloatInRange` 0.0 0.3) true)
  (`SkeletalMeshComponent.SetMorphTarget` (`self.mother3`) "Key 26" (`KismetMathLibrary.RandomFloatInRange` 0.0 0.3) true)
  (`SkeletalMeshComponent.SetMorphTarget` (`self.mother3`) "Key 27" (`KismetMathLibrary.RandomFloatInRange` 0.0 0.3) true)
  (`SkeletalMeshComponent.SetMorphTarget` (`self.mother3`) "Key 28" (`KismetMathLibrary.RandomFloatInRange` 0.0 0.3) true)
  (`SkeletalMeshComponent.SetMorphTarget` (`self.mother3`) "Key 29" (`KismetMathLibrary.RandomFloatInRange` 0.0 0.3) true)
  (`SkeletalMeshComponent.SetMorphTarget` (`self.mother3`) "Key 30" (`KismetMathLibrary.RandomFloatInRange` 0.0 0.3) true)
  (`SkeletalMeshComponent.SetMorphTarget` (`self.mother3`) "Key 31" (`KismetMathLibrary.RandomFloatInRange` 0.0 0.3) true)
  (`SkeletalMeshComponent.SetMorphTarget` (`self.mother3`) "Key 32" (`KismetMathLibrary.RandomFloatInRange` 0.0 0.3) true)
  (`SkeletalMeshComponent.SetMorphTarget` (`self.mother3`) "Key 33" (`KismetMathLibrary.RandomFloatInRange` 0.0 0.3) true)
  (`SkeletalMeshComponent.SetMorphTarget` (`self.mother3`) "Key 34" (`KismetMathLibrary.RandomFloatInRange` 0.0 0.13) true)
  (`SkeletalMeshComponent.SetMorphTarget` (`self.mother3`) "Key 35" (`KismetMathLibrary.RandomFloatInRange` 0.0 1.0) true)
  (`SkeletalMeshComponent.SetMorphTarget` (`self.mother3`) "Key 36" (`KismetMathLibrary.RandomFloatInRange` 0.0 1.0) true)
  (if (< (`KismetMathLibrary.RandomFloatInRange` 0.0 1.0) 0.5)
    (`SkeletalMeshComponent.SetMorphTarget` (`self.mother3`) "hair1" 0.0 true))
  (`SkeletalMeshComponent.SetMorphTarget` (`self.mother3`) "hair2" (`KismetMathLibrary.RandomFloatInRange` 0.0 1.0) true)
  (`SkeletalMeshComponent.SetMorphTarget` (`self.mother3`) "hair2B" (`KismetMathLibrary.RandomFloatInRange` 0.0 1.0) true)
  (bind _returnvalue (`PrimitiveComponent.CreateDynamicMaterialInstance` (`self.mother3`) 0 "/Game/Characters/Textures/Woman_Mat.Woman_Mat" "None"))
  (if (`KismetMathLibrary.RandomBool`)
    (`MaterialInstanceDynamic.SetScalarParameterValue` _returnvalue "Pants" 1.0)
    (else
      (`MaterialInstanceDynamic.SetScalarParameterValue` _returnvalue "Pants" 0.0)))
  (`MaterialInstanceDynamic.SetVectorParameterValue` _returnvalue "RandomColor" (`KismetMathLibrary.Conv_VectorToLinearColor` (`KismetMathLibrary.RandomUnitVector`)))
  (`MaterialInstanceDynamic.SetVectorParameterValue` _returnvalue "RandomColor2" (`KismetMathLibrary.Conv_VectorToLinearColor` (`KismetMathLibrary.RandomUnitVector`)))
  (if (`KismetMathLibrary.RandomBool`)
    _
    (elif (`KismetMathLibrary.RandomBool`)
      _)))

(event `NewShape`
  (goto _label))

(fn `UserConstructionScript`)